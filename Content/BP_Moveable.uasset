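; BP_Moveable is an actor that moves continuously along a looping sequence of node actors.
; Each tick it eases toward the current node by lerping its location with delta time as alpha, without sweeping.
; Within 20 units of that node it advances the index, wrapping to the first node after the last.
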(event `self.ReceiveBeginPlay`)

(event `self.ReceiveTick`
  (params (DeltaSeconds :type "Float (single-precision)"))
  (bind _returnvalue (`self.K2_GetActorLocation`))
  (bind _index (`self.Index`))
  (bind _returnvalue_2 (`self.K2_GetActorLocation` (`|GetArrayItem` (`self.Nodes`) (`self.Index`))))
  (`self.K2_SetActorLocation` (`KismetMathLibrary.VLerp` _returnvalue _returnvalue_2 DeltaSeconds))
  (if (<= (`KismetMathLibrary.Vector_Distance` _returnvalue _returnvalue_2) 20.0)
    (`/Engine/EditorBlueprintResources/StandardMacros.IncrementInt` _index
      (:`  `
        (if (>= _index (`KismetArrayLibrary.Array_Length` (`self.Nodes`)))
          (set `self.Index` 0))))))

(fn `UserConstructionScript`)