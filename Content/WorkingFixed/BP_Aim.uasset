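; BP_Aim is a patrolling enemy target that shoots and awards the player a point when destroyed.
; Each Tick it lerps toward the current entry in Nodes, looping through them as it gets close.
; It also turns Cube1 toward the player and spawns a BP_EnemyBullet at Cube's transform every frame, with no fire-rate limit.
; Overlapping an actor whose root is tagged Bullet increments WorkingPlayer's Score and destroys it.
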(event `self.ReceiveHit`
  (params (MyComp :type "PrimitiveComponent Object Reference") (Other :type "Actor Object Reference") (OtherComp :type "PrimitiveComponent Object Reference") (bSelfMoved :type Boolean) (HitLocation :type "Vector Structure") (HitNormal :type "Vector Structure") (NormalImpulse :type "Vector Structure") (Hit :type "HitResult Structure (by ref)")))

(event `self.ReceiveActorBeginOverlap`
  (params (OtherActor :type "Actor Object Reference"))
  (if (`ActorComponent.ComponentHasTag` (`Actor.RootComponent` OtherActor) "Bullet")
    (bind _asworking_player (cast `/Game/WorkingFixed/WorkingPlayer` (`GameplayStatics.GetPlayerCharacter` 0)))
    (`/Engine/EditorBlueprintResources/StandardMacros.IncrementInt` (`/Game/WorkingFixed/WorkingPlayer.Score` _asworking_player)
      (:`  `
        (`self.K2_DestroyActor`)))))

(event `self.ReceiveTick`
  (params (DeltaSeconds :type "Float (single-precision)"))
  (bind _returnvalue (`self.K2_GetActorLocation`))
  (bind _index (`self.Index`))
  (bind _returnvalue_2 (`self.K2_GetActorLocation` (`|GetArrayItem` (`self.Nodes`) (`self.Index`))))
  ;[1 1 1] Patrol
  (`self.K2_SetActorLocation` (`KismetMathLibrary.VLerp` _returnvalue _returnvalue_2 DeltaSeconds))
  ;[1 1 1] LookAT
  (`SceneComponent.K2_SetWorldRotation` (`self.Cube1`) (`KismetMathLibrary.FindLookAtRotation` (`SceneComponent.K2_GetComponentLocation` (`self.Cube1`)) (`self.K2_GetActorLocation` (`GameplayStatics.GetPlayerCharacter` 0))) false false)
  (`|SpawnActorFromClass` "/Game/WorkingFixed/BP_EnemyBullet.BP_EnemyBullet_C" (`SceneComponent.K2_GetComponentToWorld` (`self.Cube`)) "Undefined" "OverrideRootScale" null null)
  (if (<= (`KismetMathLibrary.Vector_Distance` _returnvalue _returnvalue_2) 20.0)
    (`/Engine/EditorBlueprintResources/StandardMacros.IncrementInt` _index
      (:`  `
        (if (>= _index (`KismetArrayLibrary.Array_Length` (`self.Nodes`)))
          (set `self.Index` 0))))))

(fn `UserConstructionScript`)